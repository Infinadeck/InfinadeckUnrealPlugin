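; Root Infinadeck plugin actor that integrates the omnidirectional treadmill into a level and manages its boot and shutdown.
; On BeginPlay it strips placement geometry, loads INI preferences and optionally auto-boots.
; Boot resolves camera rig and headset with fallbacks, then spawns reference objects, plus splash screen and locomotion actors when flagged.
; Tick polls InfinaKEYBIND to toggle reference visuals, boot state and treadmill, or import/reset preferences.
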(event `Key|AnyKey` :consume false
  (params (Key :type "Key Structure"))
  ;[1 0.8684 0] TO ENABLE KEYBINDS, COPY ME INTO THE EVENT GRAPH OF YOUR PLAYER PAWN AND FOLLOW BELOW INSTRUCTIONS
  (:`Pressed`
    (`GameplayStatics.GetActorOfClass` "/InfinadeckSDK/InfinaKEYBIND/InfinaKEYBIND.InfinaKEYBIND_C")))

(event `self.ReceiveBeginPlay`
  (bind _children (`SceneComponent.GetChildrenComponents` (`self.DefaultSceneRoot`) true))
  (set `self.int` 0)
  (set `self.tickcheck` true)
  (while (`self.tickcheck`)
    (if (and (`KismetSystemLibrary.IsValid` (`|GetArrayItem` _children)) (< (`self.int`) 20))
      (`/Engine/EditorBlueprintResources/StandardMacros.IncrementInt` (`self.int`)
        (:`  `
          (`ActorComponent.K2_DestroyComponent` _children)))
      (else
        (set `self.tickcheck` false))))
  (bind _returnvalue (`|SpawnActorFromClass` "/InfinadeckSDK/InfinaDATA/InfinaDATA.InfinaDATA_C" (`KismetMathLibrary.MakeTransform` (0.0 0.0 0.0)) "Undefined" "OverrideRootScale" null "" "" 1.0 60.0 null))
  (bind _output_get (set `self.preferences` _returnvalue))
  (set `/InfinadeckSDK/InfinaDATA/InfinaDATA.file_location` (`KismetStringLibrary.Concat_StrStr` (`KismetSystemLibrary.GetPlatformUserDir`) "/My Games/Infinadeck/Core/") _output_get)
  (set `/InfinadeckSDK/InfinaDATA/InfinaDATA.file_name` "infPlugin_preferences.ini" _output_get)
  (set `/InfinadeckSDK/InfinaDATA/InfinaDATA.all` (`self.default_preferences`) _output_get)
  (`/InfinadeckSDK/InfinaDATA/InfinaDATA.InitMe` _output_get)
  (if (not (`KismetSystemLibrary.IsValid` (`self.keybinds`)))
    (bind _returnvalue_2 (`GameplayStatics.GetActorOfClass` "/InfinadeckSDK/InfinaKEYBIND/InfinaKEYBIND.InfinaKEYBIND_C"))
    (bind _output_get_2 (set `self.keybinds` _returnvalue_2))
    (if (not (`KismetSystemLibrary.IsValid` _output_get_2))
      (bind _returnvalue_3 (`|SpawnActorFromClass` "/InfinadeckSDK/InfinaKEYBIND/InfinaKEYBIND.InfinaKEYBIND_C" (`KismetMathLibrary.MakeTransform` (0.0 0.0 0.0)) "Undefined" "OverrideRootScale" null null))
      (set `self.keybinds` _returnvalue_3)))
  (if (`self.auto_start`)
    (`self.Boot`)
    (else
      (`KismetSystemLibrary.PrintString` "INFINADECK NOTICE: 'Auto Start' is disabled. Please start Infinadeck Plugin by calling the Boot() function on the instance of +Infinadeck+ in your Scene." true true (struct :`R` 0.5 :`G` 1.0 :`B` 0.9 :`A` 1.0) 5.0))))

(event `self.ReceiveTick`
  (params (DeltaSeconds :type "Float (single-precision)"))
  (bind _preferences (`self.preferences`))
  (bind _preferences_2 (`self.preferences`))
  (bind _ref_objects (`self.ref_objects`))
  (bind _returnvalue (`KismetSystemLibrary.IsValid` _ref_objects))
  ;[1 1 1] InfinaKEYBIND Functions
  (bind _outbool (`/InfinadeckSDK/InfinaDATA/InfinaDATA.ReadBool` (`self.preferences`) "keyboardInputEnabled"))
  (if _outbool
    (bind _outstring (`/InfinadeckSDK/InfinaDATA/InfinaDATA.ReadString` _preferences_2 "keybindProfile"))
    (bind _outstring_2 (`/InfinadeckSDK/InfinaDATA/InfinaDATA.ReadString` _preferences_2 "customBinding"))
    (bind _out (`/InfinadeckSDK/InfinaKEYBIND/InfinaKEYBIND.GetMyKeys` (`self.keybinds`) _outstring _outstring_2))
    (set `self.my_keys` _out)
    (bind _outbool_2 (`/InfinadeckSDK/InfinaDATA/InfinaDATA.ReadBool` (`self.preferences`) "exportBindings"))
    (if _outbool_2
      (bind _output_get (set `self.keybind_names` (`|MakeArray` "Toggle Deck Ring" "Toggle Deck Edge" "Toggle Deck Center" "Toggle Reference Panel" "Toggle In-Engine Deck" "Toggle Heading" "Toggle Colorblind" "Cycle Panel Theme" "Boot/Shutdown/Reboot Plugin" "Start/Stop Treadmill" "Import Preferences" "Reset Preferences")))
      (for _index (range 12)
        (bind _out_2 (`self.LeadingZeroes` _index 2))
        (bind _output (`|GetArrayItem` _output_get _index))
        (if (`KismetStringLibrary.NotEqual_StrStr` _output)
          (bind _out_3 (`/InfinadeckSDK/InfinaKEYBIND/InfinaKEYBIND.Key2String` (`self.keybinds`) (`|GetArrayItem` (`self.my_keys`) _index)))
          (bind _returnvalue_2 (`KismetStringLibrary.Concat_StrStr` "link" _out_2))
          (`/InfinadeckSDK/InfinaDATA/InfinaDATA.Write` _preferences _returnvalue_2 (`KismetStringLibrary.Concat_StrStr` _out_3 " to " _output))
          (else
            (`/InfinadeckSDK/InfinaDATA/InfinaDATA.Write` _preferences _returnvalue_2 "---"))))
      (`/InfinadeckSDK/InfinaDATA/InfinaDATA.Write` (`self.preferences`) "exportBindings" "false"))
    (if (not (`/InfinadeckSDK/InfinaKEYBIND/InfinaKEYBIND.is_input_enabled` (`self.keybinds`)))
      (set `/InfinadeckSDK/InfinaKEYBIND/InfinaKEYBIND.is_input_enabled` true (`self.keybinds`))
      (else
        (bind _out_4 (`/InfinadeckSDK/InfinaKEYBIND/InfinaKEYBIND.KeybindRequest` (`self.keybinds`) (`self.my_keys`)))
        (switch `int` _out_4
          (:`Default`)
          (:`0`)
          (:`1`
            (if _returnvalue
              (`/InfinadeckSDK/Core/Resources/RuntimeBlueprints/InfinadeckReferenceObjects.ToggleDeckRing` _ref_objects)))
          (:`2`
            (if _returnvalue
              (`/InfinadeckSDK/Core/Resources/RuntimeBlueprints/InfinadeckReferenceObjects.ToggleDeckEdge` _ref_objects)))
          (:`3`
            (if _returnvalue
              (`/InfinadeckSDK/Core/Resources/RuntimeBlueprints/InfinadeckReferenceObjects.ToggleDeckCenter` _ref_objects)))
          (:`4`
            (if _returnvalue
              (`/InfinadeckSDK/Core/Resources/RuntimeBlueprints/InfinadeckReferenceObjects.ToggleReferencePanel` _ref_objects)))
          (:`5`
            (if _returnvalue
              (`/InfinadeckSDK/Core/Resources/RuntimeBlueprints/InfinadeckReferenceObjects.ToggleInEngineDeck` _ref_objects)))
          (:`6`
            (if _returnvalue
              (`/InfinadeckSDK/Core/Resources/RuntimeBlueprints/InfinadeckReferenceObjects.ToggleHeading` _ref_objects)))
          (:`7`
            (if _returnvalue
              (`/InfinadeckSDK/Core/Resources/RuntimeBlueprints/InfinadeckReferenceObjects.ToggleColorblind` _ref_objects)))
          (:`8`
            (if _returnvalue
              (`/InfinadeckSDK/Core/Resources/RuntimeBlueprints/InfinadeckReferenceObjects.CyclePanelTheme` _ref_objects)))
          (:`9`
            (`self.BootOrShutdown`))
          (:`10`
            (`self.StartStopTreadmill`))
          (:`11`
            (`self.ImportPreferences`))
          (:`12`
            (`self.ResetPreferences`)))))))

(fn `Boot`
  (bind _defaultsceneroot (`self.DefaultSceneRoot`))
  (bind _world_scale (`self.world_scale`))
  (bind _camera_rig (`self.camera_rig`))
  (bind _returnvalue (`self.GetParentActor` self))
  (if (not (`self.booted`))
    (set `self.booted` true)
    (if (not (`KismetSystemLibrary.IsValid` (`self.camera_rig`)))
      (`KismetSystemLibrary.PrintString` "INFINADECK NOTICE: No CameraRig Reference Assigned, Assuming Parented to CameraRig" true true (struct :`R` 0.5 :`G` 1.0 :`B` 0.9 :`A` 1.0) 5.0)
      (if (not (`KismetSystemLibrary.IsValid` _returnvalue))
        (if (`self.use_backup_camera_rig`)
          (`KismetSystemLibrary.PrintString` "INFINADECK NOTICE: No CameraRig Reference Assigned, Using InfinadeckBackupCameraRig Instead" true true (struct :`R` 0.5 :`G` 1.0 :`B` 0.9 :`A` 1.0) 5.0)
          (bind _returnvalue_2 (`|SpawnActorFromClass` "/InfinadeckSDK/Core/Resources/RuntimeBlueprints/InfinadeckBackupCameraRig.InfinadeckBackupCameraRig_C" (`KismetMathLibrary.MakeTransform` (`SceneComponent.K2_GetComponentLocation` _defaultsceneroot) (`SceneComponent.K2_GetComponentRotation` _defaultsceneroot) (`self.world_scale`)) "AlwaysSpawn" "OverrideRootScale" null null))
          (`self.K2_AttachToActor` self _returnvalue_2 "None" "SnapToTarget" "SnapToTarget" "SnapToTarget" true)
          (set `self.camera_rig` _returnvalue_2)
          (else
            (`KismetSystemLibrary.PrintString` "INFINADECK WARNING: No CameraRig Reference Assigned, Parent Null, Assuming INFINADECK is CameraRig" true true (struct :`R` 1.0 :`G` 0.5 :`A` 1.0) 5.0)
            (set `self.camera_rig` self)))
        (else
          (set `self.camera_rig` _returnvalue))))
    (if (`self.correct_position`)
      (set `self.pawnloc` "SnapToTarget")
      (else
        (set `self.pawnloc` "KeepWorld")))
    (if (`self.correct_rotation`)
      (set `self.pawnrot` "SnapToTarget")
      (else
        (set `self.pawnrot` "KeepRelative")))
    (if (`self.correct_scale`)
      (set `self.pawnscl` "SnapToTarget")
      (else
        (set `self.pawnscl` "KeepWorld")))
    (if (!= (`self.camera_rig`) self)
      (`self.K2_AttachToActor` (`self.camera_rig`) "None" (`self.pawnloc`) (`self.pawnrot`) (`self.pawnscl`)))
    (if (not (`KismetSystemLibrary.IsValid` (`self.headset`)))
      (`KismetSystemLibrary.PrintString` "INFINADECK NOTICE: No Headset Reference Assigned, Using InfinadeckAutoHeadset Instead" true true (struct :`R` 0.494711 :`G` 1.0 :`B` 0.879381 :`A` 1.0) 5.0)
      (bind _returnvalue_3 (`|SpawnActorFromClass` "/InfinadeckSDK/Core/Resources/RuntimeBlueprints/InfinadeckAutoHeadset.InfinadeckAutoHeadset_C" (`KismetMathLibrary.MakeTransform` (0.0 0.0 0.0)) "Undefined" "OverrideRootScale" null (`self.camera_rig`) null))
      (set `self.headset` _returnvalue_3))
    (if (`self.first_level`)
      (bind _returnvalue_4 (`|SpawnActorFromClass` "/InfinadeckSDK/Core/Resources/RuntimeBlueprints/InfinadeckSplashscreen.InfinadeckSplashscreen_C" (`KismetMathLibrary.MakeTransform` (`self.K2_GetActorLocation` _camera_rig) (`self.K2_GetActorRotation` _camera_rig) _world_scale) "Undefined" "OverrideRootScale" null (`self.headset`) (`self.plugin_version`) _world_scale null))
      (set `self.splash_screen` _returnvalue_4))
    (bind _returnvalue_5 (`|SpawnActorFromClass` "/InfinadeckSDK/Core/Resources/RuntimeBlueprints/InfinadeckReferenceObjects.InfinadeckReferenceObjects_C" (`KismetMathLibrary.MakeTransform` (0.0 0.0 0.0)) "Undefined" "OverrideRootScale" null null (`self.world_scale`) 0.0 60.0 null))
    (`self.K2_AttachToActor` _returnvalue_5 self "None" "SnapToTarget" "SnapToTarget" "SnapToTarget" true)
    (set `self.ref_objects` _returnvalue_5)
    (if (`self.movement_level`)
      (bind _returnvalue_6 (`|SpawnActorFromClass` "/InfinadeckSDK/Core/Resources/RuntimeBlueprints/InfinadeckLocomotion.InfinadeckLocomotion_C" (`KismetMathLibrary.MakeTransform` (0.0 0.0 0.0)) "Undefined" "OverrideRootScale" null (`self.camera_rig`) (`self.world_scale`) (`self.speed_gain`) _returnvalue_5 (`self.use_teleport`) (`self.show_collisions`) (`self.show_treadmill_velocity`) null))
      (`self.K2_AttachToActor` _returnvalue_6 self "None" "SnapToTarget" "SnapToTarget" "SnapToTarget" true)
      (set `self.infinadeck_locomotion` _returnvalue_6))
    (else
      (`KismetSystemLibrary.PrintString` "INFINADECK WARNING: Infinadeck Plugin is already booted; if manual boot is desired, un-check 'Auto Start' on the instance of +Infinadeck+ in your Scene." true true (struct :`R` 1.0 :`G` 0.5 :`A` 1.0) 5.0))))

(fn `BootOrShutdown`
  (if (`self.booted`)
    (`self.Shutdown`)
    (else
      (`self.Boot`))))

(fn `ImportPreferences`
  (`KismetSystemLibrary.PrintString` "INFINADECK: ImportPreferences" true true (struct :`R` 0.5 :`G` 1.0 :`B` 0.9 :`A` 1.0))
  (`/InfinadeckSDK/InfinaDATA/InfinaDATA.LoadSettings` (`self.preferences`))
  (`/InfinadeckSDK/InfinaDATA/InfinaDATA.LoadSettings` (`/InfinadeckSDK/Core/Resources/RuntimeBlueprints/InfinadeckReferenceObjects.preferences` (`self.ref_objects`))))

(fn `ResetPreferences`
  (bind _preferences (`self.preferences`))
  (bind _ref_objects (`self.ref_objects`))
  (bind _preferences_2 (`/InfinadeckSDK/Core/Resources/RuntimeBlueprints/InfinadeckReferenceObjects.preferences` _ref_objects))
  (`KismetSystemLibrary.PrintString` "INFINADECK: ResetPreferences()" true true (struct :`R` 0.5 :`G` 1.0 :`B` 0.9 :`A` 1.0))
  (set `/InfinadeckSDK/InfinaDATA/InfinaDATA.all` (`self.default_preferences`) _preferences)
  (set `/InfinadeckSDK/InfinaDATA/InfinaDATA.general_write_flag` true _preferences)
  (set `/InfinadeckSDK/InfinaDATA/InfinaDATA.all` (`/InfinadeckSDK/Core/Resources/RuntimeBlueprints/InfinadeckReferenceObjects.default_preferences` _ref_objects) _preferences_2)
  (set `/InfinadeckSDK/InfinaDATA/InfinaDATA.general_write_flag` true _preferences_2))

(fn `Shutdown`
  (bind _ref_objects (`self.ref_objects`))
  (bind _infinadeck_locomotion (`self.infinadeck_locomotion`))
  (bind _splash_screen (`self.splash_screen`))
  (bind _preferences (`/InfinadeckSDK/Core/Resources/RuntimeBlueprints/InfinadeckReferenceObjects.preferences` (`self.ref_objects`)))
  (if (`self.booted`)
    (if (`KismetSystemLibrary.IsValid` _preferences)
      (`self.K2_DestroyActor` _preferences))
    (if (`KismetSystemLibrary.IsValid` _ref_objects)
      (`self.K2_DestroyActor` _ref_objects))
    (if (`KismetSystemLibrary.IsValid` _splash_screen)
      (`self.K2_DestroyActor` _splash_screen))
    (if (`KismetSystemLibrary.IsValid` _infinadeck_locomotion)
      (`self.K2_DestroyActor` _infinadeck_locomotion))
    (set `self.booted` false)
    (else
      (`KismetSystemLibrary.PrintString` "INFINADECK WARNING: Infinadeck Plugin is not currently booted; shutdown request ignored." true true (struct :`R` 1.0 :`G` 0.5 :`A` 1.0) 5.0))))

(fn `StartStopTreadmill`
  (bind _returnvalue (`InfinadeckBlueprintBPLibrary.GetTreadmillRunState`))
  (if (not _returnvalue)
    (`InfinadeckBlueprintBPLibrary.StartTreadmillUserControl`)
    (else
      (`InfinadeckBlueprintBPLibrary.StopTreadmill`))))

(fn `UserConstructionScript`
  (`TextRenderComponent.K2_SetText` (`self.PluginVersionRender`) (`KismetTextLibrary.Conv_StringToText` (`self.plugin_version`))))